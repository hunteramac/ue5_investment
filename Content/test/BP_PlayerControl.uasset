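; BP_PlayerControl is a test player-control Blueprint that exposes the player UI component's context elements and actions through printed text.
; GetContext lists elements and marks the current one, while GetActions lists the current element's indexed actions.
; SetContext selects an element by tag, updating the component's current index.
; TakeAction validates an action index against that selection, then passes the action to the component's ExecuteAction.
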(event EventBeginPlay)

(event EventTick
  (params (DeltaSeconds :type Float%20%28single-precision%29)))

(fn ConstructionScript)

(fn GetContext
  (bind _component_playerui (Variables|Default|Getcomponent_playerUI))
  (LocalVariables|Setoutput " 
ContextElements: 
") ; Need a new line to correctly format in the console.
  (for (_array_element _array_index) (Variables|/Script/investment.PlayerInterface|GetContextElements _component_playerui)
    (if (== _array_index (Variables|/Script/investment.PlayerInterface|GetcurSelectedContextIndex _component_playerui))
      (LocalVariables|Setoutput (Utilities|String|Append (Utilities|String|Append (LocalVariables|Getoutput) (Utilities|String|ToString(Text) (.ElementTag (Utilities|Struct|BreakContextElementActionGroup _array_element)))) " (Current) 
"))
      (else
        ;[0.15 0.15 0.15 0.5] add elements to a textblock, to display in the console
        (LocalVariables|Setoutput (Utilities|String|Append (Utilities|String|Append (LocalVariables|Getoutput) (Utilities|String|ToString(Text) (.ElementTag (Utilities|Struct|BreakContextElementActionGroup _array_element)))) " 
")))))
  (Development|PrintString (LocalVariables|Getoutput))
  (return))

(fn GetActions
  (bind _component_playerui (Variables|Default|Getcomponent_playerUI))
  (bind _curselectedcontextindex (Variables|/Script/investment.PlayerInterface|GetcurSelectedContextIndex _component_playerui))
  (bind _contextelements (Variables|/Script/investment.PlayerInterface|GetContextElements _component_playerui))
  (bind _output (Utilities|Array|Get(acopy) _contextelements _curselectedcontextindex))
  (bind (_elementtag _actions) (Utilities|Struct|BreakContextElementActionGroup _output))
  (if (not (Utilities|Array|IsEmpty _contextelements))
    (bind _output_get (LocalVariables|SetOutput " 
Actions ("))
    (LocalVariables|SetOutput (Utilities|String|Append _output_get (Utilities|String|Append (Utilities|String|ToString(Text) _elementtag) ") 
")))
    (for (_array_element _array_index) _actions
      (LocalVariables|SetOutput (Utilities|String|Append (Utilities|String|Append (Utilities|String|Append (Utilities|String|Append (LocalVariables|GetOutput) (Utilities|String|ToString(Integer) _array_index)) ". ") (Utilities|String|ToString(Text) (.entryText (Utilities|Struct|BreakListEntry _array_element)))) " 
")))
    (Development|PrintString (LocalVariables|GetOutput))))

(fn SetContext
  (params (Tag :type Text))
  (bind _returnvalue (Utilities|String|ToString(Text) Tag))
  (bind _component_playerui (Variables|Default|Getcomponent_playerUI))
  (bind (_array_element _array_index) (Utilities|Array|ForEachLoopwithBreak (Variables|/Script/investment.PlayerInterface|GetContextElements _component_playerui) :!label _label)
    (:LoopBody
      (if (Utilities|Enum|Equal(Enum) (Utilities|String|ToString(Text) (.ElementTag (Utilities|Struct|BreakContextElementActionGroup _array_element))) (Utilities|String|ToString(Text) Tag))
        (LocalVariables|SetNewLocalVar _array_index)
        (goto _label Break)))
    (:Completed
      (if (== (LocalVariables|GetNewLocalVar) -1)
        (Development|PrintString (Utilities|String|Append _returnvalue (Utilities|String|MakeLiteralString "| Context Element not found.")))
        (else
          (Variables|/Script/investment.PlayerInterface|SetcurSelectedContextIndex _component_playerui (LocalVariables|GetNewLocalVar))
          (Development|PrintString (Utilities|String|Append (Utilities|String|MakeLiteralString "Set Context | ") _returnvalue)))))))

(fn TakeAction
  (params (ActionIndex :type Integer))
  (bind _component_playerui (Variables|Default|Getcomponent_playerUI))
  (bind _contextelements (Variables|/Script/investment.PlayerInterface|GetContextElements _component_playerui))
  (bind _curselectedcontextindex (Variables|/Script/investment.PlayerInterface|GetcurSelectedContextIndex _component_playerui))
  (bind _output (Utilities|Array|Get(acopy) _contextelements _curselectedcontextindex))
  (bind _actions (Utilities|Struct|BreakContextElementActionGroup _output))
  (if (Utilities|Array|IsEmpty _contextelements)
    (Development|PrintString "Invalid action" :!label _label)
    (elif (Utilities|Array|IsValidIndex _contextelements _curselectedcontextindex)
      (if (Utilities|Array|IsEmpty _actions)
        (goto _label)
        (elif (Utilities|Array|IsValidIndex _actions ActionIndex)
          (Development|PrintString "outcome: 
")
          (Class|PlayerInterface|ExecuteAction (Variables|Default|Getcomponent_playerUI) (Utilities|Array|Get(acopy) _actions ActionIndex))
          (else
            (goto _label))))
      (else
        (goto _label)))))